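; Actor that builds a VCR-style date and time stamp from its time and date variables.
; It splits the values into digits, with optional 12-hour AM/PM, and writes them to Time_stamp_MPC, then adds static-mesh digits alongside a scene capture.
; RunTimeEnable moves this from the Construction Script to a one-second delayed Tick, which adds new components each pass without removing old ones.
; That Tick always nudges the root along X and back.
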(event EventBeginPlay)

(event Collision|EventActorBeginOverlap
  (params (OtherActor :type Actor%20Object%20Reference)))

(event EventTick
  (params (DeltaSeconds :type Float%20%28single-precision%29))
  (bind _defaultsceneroot (Variables|Default|GetDefaultSceneRoot))
  (bind _year__4_digit_max_ (Variables|Default|GetYear%20%284%20digit%20max%29))
  (bind _hour (Variables|Default|GetHour))
  (bind _hour_2 (Variables|Default|GetHour))
  (bind _minute (Variables|Default|GetMinute))
  (bind _day (Variables|Default|GetDay))
  (bind _returnvalue (Math|Conversions|ToFloat(Integer) _hour_2))
  (bind _returnvalue_2 (Math|Conversions|ToFloat(Integer) _hour))
  (bind _returnvalue_3 (Transformation|GetWorldLocation _defaultsceneroot))
  (bind _returnvalue_4 (Math|Conversions|ToFloat(Integer) _minute))
  (bind _returnvalue_5 (Math|Conversions|ToFloat(Integer) _day))
  (bind _returnvalue_6 (Math|Conversions|ToFloat(Integer) _year__4_digit_max_))
  (bind _returnvalue_7 (Transformation|GetWorldLocation _defaultsceneroot))
  (bind _remainder (Math|Float|Division(WholeandRemainder) _returnvalue_2 1e+01))
  (bind _remainder_2 (Math|Float|Division(WholeandRemainder) _returnvalue 1e+01))
  (bind (_x _y _z) (Math|Vector|BreakVector _returnvalue_3))
  (bind (_remainder_3 _returnvalue_8) (Math|Float|Division(WholeandRemainder) _returnvalue_4 1e+01))
  (bind (_remainder_4 _returnvalue_9) (Math|Float|Division(WholeandRemainder) _returnvalue_5 1e+01))
  (bind (_remainder_5 _returnvalue_10) (Math|Float|Division(WholeandRemainder) _returnvalue_6 1e+03))
  (bind _returnvalue_11 (- _returnvalue_2 12.0))
  (bind (_x_2 _y_2 _z_2) (Math|Vector|BreakVector _returnvalue_7))
  (bind _remainder_6 (Math|Float|Division(WholeandRemainder) _returnvalue_11 1e+01))
  (bind (_remainder_7 _returnvalue_12) (Math|Float|Division(WholeandRemainder) _remainder_5 1e+02))
  (bind (_remainder_8 _returnvalue_13) (Math|Float|Division(WholeandRemainder) _remainder_7 1e+01))
  (Utilities|FlowControl|Delay 1.0)
  (Transformation|SetWorldLocation _defaultsceneroot (Math|Vector|MakeVector (+ _x_2 1.0) _y_2 _z_2) false false)
  (Transformation|SetWorldLocation _defaultsceneroot (Math|Vector|MakeVector (- _x 1.0) _y _z) false false)
  (if (Variables|Default|GetRunTime%20Enable)
    (AddComponent|AddSceneCaptureComponent2D false)
    ;[1 1 1] AM PM visible
    (if (Variables|Default|Get12h/24h%20switch)
      (Rendering|Material|SetScalarParameterValue "/Game/CRT_VCR_Material/Materials/T_Trace/BP_TS_Materials/time_stamp_MPC.time_stamp_MPC" "AM/PM visible" 1.0 :!class /Script/Engine.KismetMaterialLibrary)
      (if (< (Variables|Default|GetHour) 12)
        (Variables|Default|SetAM/PM%20Value 1e+01)
        (else
          (Variables|Default|SetAM/PM%20Value 11.0)))
      (Rendering|Material|SetScalarParameterValue "/Game/CRT_VCR_Material/Materials/T_Trace/BP_TS_Materials/time_stamp_MPC.time_stamp_MPC" "AM_PM" (Variables|Default|GetAM/PM%20Value) :!class /Script/Engine.KismetMaterialLibrary)
      ;[1 1 1] 12H / 24H
      (if (and (or (< _hour 10) (> _hour 12)) (< _hour 22))
        (Rendering|Material|SetScalarParameterValue "/Game/CRT_VCR_Material/Materials/T_Trace/BP_TS_Materials/time_stamp_MPC.time_stamp_MPC" "HD1_enabled" 0.0 :!class /Script/Engine.KismetMaterialLibrary)
        (Rendering|Material|SetScalarParameterValue "/Game/CRT_VCR_Material/Materials/T_Trace/BP_TS_Materials/time_stamp_MPC.time_stamp_MPC" "HD2_time_offset" (.Remainder (Math|Float|Division(WholeandRemainder) (Math|Conversions|ToFloat(Integer) _hour) 12.0)) :!class /Script/Engine.KismetMaterialLibrary)
        (else
          (Rendering|Material|SetScalarParameterValue "/Game/CRT_VCR_Material/Materials/T_Trace/BP_TS_Materials/time_stamp_MPC.time_stamp_MPC" "HD1_enabled" 1.0 :!class /Script/Engine.KismetMaterialLibrary)
          (if (> _hour 21)
            (Rendering|Material|SetScalarParameterValue "/Game/CRT_VCR_Material/Materials/T_Trace/BP_TS_Materials/time_stamp_MPC.time_stamp_MPC" "HD1_time_offset" (Math|Conversions|ToFloat(Integer) (/ (Math|Float|Truncate (- _returnvalue_11 _remainder_6)) 10)) :!class /Script/Engine.KismetMaterialLibrary)
            (Rendering|Material|SetScalarParameterValue "/Game/CRT_VCR_Material/Materials/T_Trace/BP_TS_Materials/time_stamp_MPC.time_stamp_MPC" "HD2_time_offset" _remainder_6 :!class /Script/Engine.KismetMaterialLibrary)
            (else
              (Rendering|Material|SetScalarParameterValue "/Game/CRT_VCR_Material/Materials/T_Trace/BP_TS_Materials/time_stamp_MPC.time_stamp_MPC" "HD1_time_offset" (Math|Conversions|ToFloat(Integer) (/ (- _hour (Math|Float|Truncate _remainder)) 10)) :!class /Script/Engine.KismetMaterialLibrary)
              (Rendering|Material|SetScalarParameterValue "/Game/CRT_VCR_Material/Materials/T_Trace/BP_TS_Materials/time_stamp_MPC.time_stamp_MPC" "HD2_time_offset" _remainder :!class /Script/Engine.KismetMaterialLibrary)))))
      (else
        (Rendering|Material|SetScalarParameterValue "/Game/CRT_VCR_Material/Materials/T_Trace/BP_TS_Materials/time_stamp_MPC.time_stamp_MPC" "AM/PM visible" 0.0 :!class /Script/Engine.KismetMaterialLibrary)
        (if (or (< _hour_2 10) (> _hour_2 23))
          (Rendering|Material|SetScalarParameterValue "/Game/CRT_VCR_Material/Materials/T_Trace/BP_TS_Materials/time_stamp_MPC.time_stamp_MPC" "HD1_enabled" 0.0 :!class /Script/Engine.KismetMaterialLibrary)
          (Rendering|Material|SetScalarParameterValue "/Game/CRT_VCR_Material/Materials/T_Trace/BP_TS_Materials/time_stamp_MPC.time_stamp_MPC" "HD2_time_offset" (.Remainder (Math|Float|Division(WholeandRemainder) (Math|Conversions|ToFloat(Integer) _hour_2) 24.0)) :!class /Script/Engine.KismetMaterialLibrary)
          (else
            (Rendering|Material|SetScalarParameterValue "/Game/CRT_VCR_Material/Materials/T_Trace/BP_TS_Materials/time_stamp_MPC.time_stamp_MPC" "HD1_enabled" 1.0 :!class /Script/Engine.KismetMaterialLibrary)
            (Rendering|Material|SetScalarParameterValue "/Game/CRT_VCR_Material/Materials/T_Trace/BP_TS_Materials/time_stamp_MPC.time_stamp_MPC" "HD1_time_offset" (Math|Conversions|ToFloat(Integer) (/ (- _hour_2 (Math|Float|Truncate _remainder_2)) 10)) :!class /Script/Engine.KismetMaterialLibrary)
            (Rendering|Material|SetScalarParameterValue "/Game/CRT_VCR_Material/Materials/T_Trace/BP_TS_Materials/time_stamp_MPC.time_stamp_MPC" "HD2_time_offset" _remainder_2 :!class /Script/Engine.KismetMaterialLibrary)))))
    ;[1 1 1] Minute
    (Rendering|Material|SetScalarParameterValue "/Game/CRT_VCR_Material/Materials/T_Trace/BP_TS_Materials/time_stamp_MPC.time_stamp_MPC" "Min1_time_offset" (Math|Conversions|ToFloat(Integer) _returnvalue_8) :!class /Script/Engine.KismetMaterialLibrary)
    (Rendering|Material|SetScalarParameterValue "/Game/CRT_VCR_Material/Materials/T_Trace/BP_TS_Materials/time_stamp_MPC.time_stamp_MPC" "Min2_time_offset" _remainder_3 :!class /Script/Engine.KismetMaterialLibrary)
    ;[1 1 1] MM/DD/YYYY
    (Rendering|Material|SetScalarParameterValue "/Game/CRT_VCR_Material/Materials/T_Trace/BP_TS_Materials/time_stamp_MPC.time_stamp_MPC" "Month" (Math|Conversions|ToFloat(Integer) (Variables|Default|GetMonth)) :!class /Script/Engine.KismetMaterialLibrary)
    (Rendering|Material|SetScalarParameterValue "/Game/CRT_VCR_Material/Materials/T_Trace/BP_TS_Materials/time_stamp_MPC.time_stamp_MPC" "day_digit1" (Math|Conversions|ToFloat(Integer) _returnvalue_9) :!class /Script/Engine.KismetMaterialLibrary)
    (Rendering|Material|SetScalarParameterValue "/Game/CRT_VCR_Material/Materials/T_Trace/BP_TS_Materials/time_stamp_MPC.time_stamp_MPC" "day_digit2" _remainder_4 :!class /Script/Engine.KismetMaterialLibrary)
    (Rendering|Material|SetScalarParameterValue "/Game/CRT_VCR_Material/Materials/T_Trace/BP_TS_Materials/time_stamp_MPC.time_stamp_MPC" "Year1" (Math|Conversions|ToFloat(Integer) _returnvalue_10) :!class /Script/Engine.KismetMaterialLibrary)
    (Rendering|Material|SetScalarParameterValue "/Game/CRT_VCR_Material/Materials/T_Trace/BP_TS_Materials/time_stamp_MPC.time_stamp_MPC" "Year2" (Math|Conversions|ToFloat(Integer) _returnvalue_12) :!class /Script/Engine.KismetMaterialLibrary)
    (Rendering|Material|SetScalarParameterValue "/Game/CRT_VCR_Material/Materials/T_Trace/BP_TS_Materials/time_stamp_MPC.time_stamp_MPC" "Year3" (Math|Conversions|ToFloat(Integer) _returnvalue_13) :!class /Script/Engine.KismetMaterialLibrary)
    (Rendering|Material|SetScalarParameterValue "/Game/CRT_VCR_Material/Materials/T_Trace/BP_TS_Materials/time_stamp_MPC.time_stamp_MPC" "Year4" _remainder_8 :!class /Script/Engine.KismetMaterialLibrary)
    ;[1 1 1] Digits
    (AddComponent|AddStaticMeshComponent false)
    (AddComponent|AddStaticMeshComponent false)
    (AddComponent|AddStaticMeshComponent false)
    (AddComponent|AddStaticMeshComponent false)
    (AddComponent|AddStaticMeshComponent false)
    (AddComponent|AddStaticMeshComponent false)
    (AddComponent|AddStaticMeshComponent false)
    (AddComponent|AddStaticMeshComponent false)
    (AddComponent|AddStaticMeshComponent false)
    (AddComponent|AddStaticMeshComponent false)
    (AddComponent|AddStaticMeshComponent false)
    (AddComponent|AddStaticMeshComponent false)
    (AddComponent|AddStaticMeshComponent false)
    (AddComponent|AddStaticMeshComponent false)
    (AddComponent|AddStaticMeshComponent false)
    (AddComponent|AddStaticMeshComponent false)
    (AddComponent|AddStaticMeshComponent false)
    (AddComponent|AddStaticMeshComponent false)))

(fn ConstructionScript
  (bind _year__4_digit_max_ (Variables|Default|GetYear%20%284%20digit%20max%29))
  (bind _hour (Variables|Default|GetHour))
  (bind _hour_2 (Variables|Default|GetHour))
  (bind _minute (Variables|Default|GetMinute))
  (bind _day (Variables|Default|GetDay))
  (bind _returnvalue (Math|Conversions|ToFloat(Integer) _hour_2))
  (bind _returnvalue_2 (Math|Conversions|ToFloat(Integer) _hour))
  (bind _returnvalue_3 (Math|Conversions|ToFloat(Integer) _minute))
  (bind _returnvalue_4 (Math|Conversions|ToFloat(Integer) _day))
  (bind _returnvalue_5 (Math|Conversions|ToFloat(Integer) _year__4_digit_max_))
  (bind _remainder (Math|Float|Division(WholeandRemainder) _returnvalue_2 1e+01))
  (bind _remainder_2 (Math|Float|Division(WholeandRemainder) _returnvalue 1e+01))
  (bind (_remainder_3 _returnvalue_6) (Math|Float|Division(WholeandRemainder) _returnvalue_3 1e+01))
  (bind (_remainder_4 _returnvalue_7) (Math|Float|Division(WholeandRemainder) _returnvalue_4 1e+01))
  (bind (_remainder_5 _returnvalue_8) (Math|Float|Division(WholeandRemainder) _returnvalue_5 1e+03))
  (bind _returnvalue_9 (- _returnvalue_2 12.0))
  (bind _remainder_6 (Math|Float|Division(WholeandRemainder) _returnvalue_9 1e+01))
  (bind (_remainder_7 _returnvalue_10) (Math|Float|Division(WholeandRemainder) _remainder_5 1e+02))
  (bind (_remainder_8 _returnvalue_11) (Math|Float|Division(WholeandRemainder) _remainder_7 1e+01))
  (if (not (Variables|Default|GetRunTime%20Enable))
    (AddComponent|AddSceneCaptureComponent2D false)
    ;[1 1 1] AM PM visible
    (if (Variables|Default|Get12h/24h%20switch)
      (Rendering|Material|SetScalarParameterValue "/Game/CRT_VCR_Material/Materials/T_Trace/BP_TS_Materials/time_stamp_MPC.time_stamp_MPC" "AM/PM visible" 1.0 :!class /Script/Engine.KismetMaterialLibrary)
      (if (< (Variables|Default|GetHour) 12)
        (Variables|Default|SetAM/PM%20Value 1e+01)
        (else
          (Variables|Default|SetAM/PM%20Value 11.0)))
      (Rendering|Material|SetScalarParameterValue "/Game/CRT_VCR_Material/Materials/T_Trace/BP_TS_Materials/time_stamp_MPC.time_stamp_MPC" "AM_PM" (Variables|Default|GetAM/PM%20Value) :!class /Script/Engine.KismetMaterialLibrary)
      ;[1 1 1] 12H / 24H
      (if (and (or (< _hour 10) (> _hour 12)) (< _hour 22))
        (Rendering|Material|SetScalarParameterValue "/Game/CRT_VCR_Material/Materials/T_Trace/BP_TS_Materials/time_stamp_MPC.time_stamp_MPC" "HD1_enabled" 0.0 :!class /Script/Engine.KismetMaterialLibrary)
        (Rendering|Material|SetScalarParameterValue "/Game/CRT_VCR_Material/Materials/T_Trace/BP_TS_Materials/time_stamp_MPC.time_stamp_MPC" "HD2_time_offset" (.Remainder (Math|Float|Division(WholeandRemainder) (Math|Conversions|ToFloat(Integer) _hour) 12.0)) :!class /Script/Engine.KismetMaterialLibrary)
        (else
          (Rendering|Material|SetScalarParameterValue "/Game/CRT_VCR_Material/Materials/T_Trace/BP_TS_Materials/time_stamp_MPC.time_stamp_MPC" "HD1_enabled" 1.0 :!class /Script/Engine.KismetMaterialLibrary)
          (if (> _hour 21)
            (Rendering|Material|SetScalarParameterValue "/Game/CRT_VCR_Material/Materials/T_Trace/BP_TS_Materials/time_stamp_MPC.time_stamp_MPC" "HD1_time_offset" (Math|Conversions|ToFloat(Integer) (/ (Math|Float|Truncate (- _returnvalue_9 _remainder_6)) 10)) :!class /Script/Engine.KismetMaterialLibrary)
            (Rendering|Material|SetScalarParameterValue "/Game/CRT_VCR_Material/Materials/T_Trace/BP_TS_Materials/time_stamp_MPC.time_stamp_MPC" "HD2_time_offset" _remainder_6 :!class /Script/Engine.KismetMaterialLibrary)
            (else
              (Rendering|Material|SetScalarParameterValue "/Game/CRT_VCR_Material/Materials/T_Trace/BP_TS_Materials/time_stamp_MPC.time_stamp_MPC" "HD1_time_offset" (Math|Conversions|ToFloat(Integer) (/ (- _hour (Math|Float|Truncate _remainder)) 10)) :!class /Script/Engine.KismetMaterialLibrary)
              (Rendering|Material|SetScalarParameterValue "/Game/CRT_VCR_Material/Materials/T_Trace/BP_TS_Materials/time_stamp_MPC.time_stamp_MPC" "HD2_time_offset" _remainder :!class /Script/Engine.KismetMaterialLibrary)))))
      (else
        (Rendering|Material|SetScalarParameterValue "/Game/CRT_VCR_Material/Materials/T_Trace/BP_TS_Materials/time_stamp_MPC.time_stamp_MPC" "AM/PM visible" 0.0 :!class /Script/Engine.KismetMaterialLibrary)
        (if (or (< _hour_2 10) (> _hour_2 23))
          (Rendering|Material|SetScalarParameterValue "/Game/CRT_VCR_Material/Materials/T_Trace/BP_TS_Materials/time_stamp_MPC.time_stamp_MPC" "HD1_enabled" 0.0 :!class /Script/Engine.KismetMaterialLibrary)
          (Rendering|Material|SetScalarParameterValue "/Game/CRT_VCR_Material/Materials/T_Trace/BP_TS_Materials/time_stamp_MPC.time_stamp_MPC" "HD2_time_offset" (.Remainder (Math|Float|Division(WholeandRemainder) (Math|Conversions|ToFloat(Integer) _hour_2) 24.0)) :!class /Script/Engine.KismetMaterialLibrary)
          (else
            (Rendering|Material|SetScalarParameterValue "/Game/CRT_VCR_Material/Materials/T_Trace/BP_TS_Materials/time_stamp_MPC.time_stamp_MPC" "HD1_enabled" 1.0 :!class /Script/Engine.KismetMaterialLibrary)
            (Rendering|Material|SetScalarParameterValue "/Game/CRT_VCR_Material/Materials/T_Trace/BP_TS_Materials/time_stamp_MPC.time_stamp_MPC" "HD1_time_offset" (Math|Conversions|ToFloat(Integer) (/ (- _hour_2 (Math|Float|Truncate _remainder_2)) 10)) :!class /Script/Engine.KismetMaterialLibrary)
            (Rendering|Material|SetScalarParameterValue "/Game/CRT_VCR_Material/Materials/T_Trace/BP_TS_Materials/time_stamp_MPC.time_stamp_MPC" "HD2_time_offset" _remainder_2 :!class /Script/Engine.KismetMaterialLibrary)))))
    ;[1 1 1] Minute
    (Rendering|Material|SetScalarParameterValue "/Game/CRT_VCR_Material/Materials/T_Trace/BP_TS_Materials/time_stamp_MPC.time_stamp_MPC" "Min1_time_offset" (Math|Conversions|ToFloat(Integer) _returnvalue_6) :!class /Script/Engine.KismetMaterialLibrary)
    (Rendering|Material|SetScalarParameterValue "/Game/CRT_VCR_Material/Materials/T_Trace/BP_TS_Materials/time_stamp_MPC.time_stamp_MPC" "Min2_time_offset" _remainder_3 :!class /Script/Engine.KismetMaterialLibrary)
    ;[1 1 1] MM/DD/YYYY
    (Rendering|Material|SetScalarParameterValue "/Game/CRT_VCR_Material/Materials/T_Trace/BP_TS_Materials/time_stamp_MPC.time_stamp_MPC" "Month" (Math|Conversions|ToFloat(Integer) (Variables|Default|GetMonth)) :!class /Script/Engine.KismetMaterialLibrary)
    (Rendering|Material|SetScalarParameterValue "/Game/CRT_VCR_Material/Materials/T_Trace/BP_TS_Materials/time_stamp_MPC.time_stamp_MPC" "day_digit1" (Math|Conversions|ToFloat(Integer) _returnvalue_7) :!class /Script/Engine.KismetMaterialLibrary)
    (Rendering|Material|SetScalarParameterValue "/Game/CRT_VCR_Material/Materials/T_Trace/BP_TS_Materials/time_stamp_MPC.time_stamp_MPC" "day_digit2" _remainder_4 :!class /Script/Engine.KismetMaterialLibrary)
    (Rendering|Material|SetScalarParameterValue "/Game/CRT_VCR_Material/Materials/T_Trace/BP_TS_Materials/time_stamp_MPC.time_stamp_MPC" "Year1" (Math|Conversions|ToFloat(Integer) _returnvalue_8) :!class /Script/Engine.KismetMaterialLibrary)
    (Rendering|Material|SetScalarParameterValue "/Game/CRT_VCR_Material/Materials/T_Trace/BP_TS_Materials/time_stamp_MPC.time_stamp_MPC" "Year2" (Math|Conversions|ToFloat(Integer) _returnvalue_10) :!class /Script/Engine.KismetMaterialLibrary)
    (Rendering|Material|SetScalarParameterValue "/Game/CRT_VCR_Material/Materials/T_Trace/BP_TS_Materials/time_stamp_MPC.time_stamp_MPC" "Year3" (Math|Conversions|ToFloat(Integer) _returnvalue_11) :!class /Script/Engine.KismetMaterialLibrary)
    (Rendering|Material|SetScalarParameterValue "/Game/CRT_VCR_Material/Materials/T_Trace/BP_TS_Materials/time_stamp_MPC.time_stamp_MPC" "Year4" _remainder_8 :!class /Script/Engine.KismetMaterialLibrary)
    ;[1 1 1] Digits
    (AddComponent|AddStaticMeshComponent false)
    (AddComponent|AddStaticMeshComponent false)
    (AddComponent|AddStaticMeshComponent false)
    (AddComponent|AddStaticMeshComponent false)
    (AddComponent|AddStaticMeshComponent false)
    (AddComponent|AddStaticMeshComponent false)
    (AddComponent|AddStaticMeshComponent false)
    (AddComponent|AddStaticMeshComponent false)
    (AddComponent|AddStaticMeshComponent false)
    (AddComponent|AddStaticMeshComponent false)
    (AddComponent|AddStaticMeshComponent false)
    (AddComponent|AddStaticMeshComponent false)
    (AddComponent|AddStaticMeshComponent false)
    (AddComponent|AddStaticMeshComponent false)
    (AddComponent|AddStaticMeshComponent false)
    (AddComponent|AddStaticMeshComponent false)
    (AddComponent|AddStaticMeshComponent false)
    (AddComponent|AddStaticMeshComponent false)))